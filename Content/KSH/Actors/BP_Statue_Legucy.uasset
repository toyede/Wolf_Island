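; Legacy boss-fight statue that staggers and damages the boss when it runs into the statue.
; On capsule overlap, Interact checks for the Boss tag and asks the boss AI controller to enter Groggy.
; If that succeeds, the statue destroys itself and deals damage to the boss.
; An overlap-end handler meant to re-enable statue summoning remains, but its boss lookup and binding are disconnected.
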(event `OnStatueOverlapEnd_Event`
  (bind _asaic_enemy_ai_boss (cast `/Game/KSH/AI/Controllers/AIC_EnemyAI_Boss` (`AIBlueprintHelperLibrary.GetAIController` null)))
  (if (`|EnumEquality` (cast `EBossState` (`BlackboardComponent.GetValueAsEnum` (`AIController.Blackboard` _asaic_enemy_ai_boss) (`self.StateKey`))) "Groggy")
    (set `/Game/KSH/AI/BP_EnemyAI_Boss_legacy.bCanSummonStatue` true (`self.Boss`))
    (`self.K2_DestroyActor`)))

(event `self.Capsule.OnComponentBeginOverlap`
  (params (OverlappedComponent :type "PrimitiveComponent Object Reference") (OtherActor :type "Actor Object Reference") (OtherComp :type "PrimitiveComponent Object Reference") (OtherBodyIndex :type Integer) (bFromSweep :type Boolean) (SweepResult :type "HitResult Structure (by ref)"))
  (`self.Interact` OtherActor (`AIBlueprintHelperLibrary.GetAIController` OtherActor)))

(fn `Interact`
  (params (Actor :type "Actor Object Reference") (AIC :type "AIController Object Reference"))
  (if (`self.ActorHasTag` Actor "Boss")
    (bind _asaic_enemy_ai_boss (cast `/Game/KSH/AI/Controllers/AIC_EnemyAI_Boss` AIC))
    (bind _returnvalue (`EnemyAIBossController.SetStateAsGroggy` _asaic_enemy_ai_boss))
    (if (`|EnumEquality` _returnvalue "Groggy")
      (`self.K2_DestroyActor`)
      (`GameplayStatics.ApplyDamage` Actor 20.0))
    (return)))

(fn `UserConstructionScript`)