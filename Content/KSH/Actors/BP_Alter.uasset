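; BP_Alter is an interactable altar actor that stuns the boss when used and is then destroyed.
; On Interact it finds the BP_EnemyAI_Boss_legacy instance and sets its CanSummonAlter flag, both on the boss and in its Blackboard.
; It writes the Stun state to the Blackboard, calls SetstateAsStun on AIC_EnemyAI_Boss, then destroys itself.
; A cast of the interactor to BP_MainPlayer is left unconnected.
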(event `self.Interact`
  (params (Interactor :type "Actor Object Reference"))
  (`KismetSystemLibrary.PrintString` "Alter Interacted")
  (bind _returnvalue (`GameplayStatics.GetActorOfClass` "/Game/KSH/AI/BP_EnemyAI_Boss_legacy.BP_EnemyAI_Boss_legacy_C"))
  (bind _output_get (set `self.BossRef` _returnvalue))
  (set `/Game/KSH/AI/BP_EnemyAI_Boss_legacy.bCanSummonAlter` true _output_get)
  (bind _aicontroller (`/Game/KSH/AI/BP_EnemyAI_Boss_legacy.AIController` _output_get))
  (bind _blackboard (`AIController.Blackboard` _aicontroller))
  (`BlackboardComponent.SetValueAsBool` _blackboard "bCanSummonAlter" true)
  (`BlackboardComponent.SetValueAsEnum` _blackboard "State" (enumliteral `EBossState` "Stun"))
  (bind _asaic_enemy_ai_boss (cast `/Game/KSH/AI/Controllers/AIC_EnemyAI_Boss` _aicontroller))
  (`/Game/KSH/AI/Controllers/AIC_EnemyAI_Boss.SetstateAsStun` _asaic_enemy_ai_boss)
  (`self.K2_DestroyActor`))

(fn `UserConstructionScript`)