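; Legacy boss enemy with claw attack, rush, statue and altar summons, groggy, stun and death actions.
; Actions mostly signal completion through dispatchers, while Blackboard keys carry the Dead state and summon availability to the AI.
; Claw hits use a notify-timed sphere trace; rush launches with zeroed friction and a temporary damage capsule.
; Statues spawn at random spline points, altars at a set actor; timers remove both and re-enable summoning.
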(event `Attack`
  ; Attack
  (`GameplayStatics.PlaySoundAtLocation` "/Game/Fab/Sound/Enemy/Boss_Attack.Boss_Attack" (`self.K2_GetActorLocation`) (struct) 1.0 1.0 0.0 "/Game/KSH/Sounds/Attenuation/SA_AISoundRange.SA_AISoundRange" null null null)
  (bind _notifyname (`|PlayMontage` (`self.Mesh`) "/Game/KSH/Animations/Montages/AM_Claw.AM_Claw")
    (:`OnNotifyBegin`
      (switch `name` _notifyname
        (:`Attack`
          (bind _outhit (`KismetSystemLibrary.SphereTraceSingleForObjects` :`Start` (+ (`self.K2_GetActorLocation`) (* (`self.GetActorForwardVector`) 100.0)) :`End` (+ (`self.K2_GetActorLocation`) (* (`self.GetActorForwardVector`) 250.0)) :`Radius` 20.0 :`ObjectTypes` (`|MakeArray` "ObjectTypeQuery3" :!type "EObjectTypeQuery Enum") :`DrawDebugType` "ForDuration"))
          (if true
            (`GameplayStatics.ApplyDamage` (`.HitActor` (`GameplayStatics.BreakHitResult` _outhit)) (`self.AttackDamage`) (`self.GetController`) self)))))))

(event `self.ReceivePossessed`
  (params (NewController :type "Controller Object Reference"))
  ; Possessed
  (bind _asaicontroller (cast `AIController` (`self.GetController`)))
  (set `self.AIController` _asaicontroller))

(event `self.ReceiveAnyDamage`
  (params (Damage :type "Float (single-precision)") (DamageType :type "DamageType Object Reference") (InstigatedBy :type "Controller Object Reference") (DamageCauser :type "Actor Object Reference"))
  (bind _statuscomponent (`self.StatusComponent`))
  ; Damage
  (`StatusComponent.DecreaseHP` _statuscomponent Damage)
  (if (<= (`StatusComponent.CurrentHP` _statuscomponent) 0.0)
    (`BlackboardComponent.SetValueAsEnum` (`AIController.Blackboard` (`self.AIController`)) "State" (enumliteral `EBossState` "Dead"))))

(event `Groggy`
  ; Groggy
  (`|PlayMontage` (`self.Mesh`) "/Game/KSH/Animations/Montages/AM_KnockedDown.AM_KnockedDown"
    (:`OnCompleted`
      _)
    (:`OnInterrupted`
      _))
  (`self.OnGroggyEnd`))

(event `Die`
  ; Die
  (`GameplayStatics.PlaySoundAtLocation` "/Game/Fab/Sound/Enemy/Boss_Die.Boss_Die" (`self.K2_GetActorLocation`) (struct) 1.0 1.0 0.0 "/Game/KSH/Sounds/Attenuation/SA_AISoundRange.SA_AISoundRange" null null null)
  (`AnimInstance.Montage_Stop` (`SkeletalMeshComponent.GetAnimInstance` (`self.Mesh`)) 0.1 null)
  (`self.OnDieEnd`))

(event `SummonStatue`
  (bind _statuelocation (`self.StatueLocation`))
  (bind _locations (`/Game/KSH/Actors/BP_StatueSpawnLocation.Locations` (`self.SpawnStatueLocation`)))
  ; SummonStatue
  (`GameplayStatics.PlaySoundAtLocation` "/Game/Fab/Sound/Enemy/Boss_Roar.Boss_Roar" (`self.K2_GetActorLocation`) (struct) 1.0 1.0 0.0 "/Game/KSH/Sounds/Attenuation/SA_AISoundRange.SA_AISoundRange" null null null)
  (`|PlayMontage` (`self.Mesh`) "/Game/KSH/Animations/Montages/AM_SummonStatue.AM_SummonStatue"
    (:`OnCompleted`
      _)
    (:`OnInterrupted`
      _))
  (`self.OnSummonStatueEnd`)
  (set `self.StatueLocation` (`SplineComponent.GetLocationAtSplinePoint` _locations (`KismetMathLibrary.RandomIntegerInRange` 0 (- (`SplineComponent.GetNumberOfSplinePoints` _locations) 1)) "World"))
  (bind _returnvalue (`|SpawnActorFromClass` "/Game/KSH/Actors/BP_Statue_Legucy.BP_Statue_Legucy_C" (`KismetMathLibrary.MakeTransform` _statuelocation) "Undefined" "MultiplyWithRoot" null null))
  (`KismetSystemLibrary.Delay` 0.2)
  (`GameplayStatics.SpawnEmitterAtLocation` "/Game/StarterContent/Particles/P_Explosion.P_Explosion" _statuelocation (struct) (10.0 10.0 10.0))
  (set `self.bCanSummonStatue` false)
  (`BlackboardComponent.SetValueAsBool` (`AIController.Blackboard` (`self.AIController`)) "bCanSummonStatue" false)
  (`KismetSystemLibrary.K2_SetTimerDelegate` (delegate `AutoDeleteStatue`) 30.0))

(event `Rush`
  ; Rush
  (`GameplayStatics.PlaySoundAtLocation` "/Game/Fab/Sound/Enemy/Boss_Rush.Boss_Rush" (`self.K2_GetActorLocation`) (struct) 1.0 1.0 0.0 "/Game/KSH/Sounds/Attenuation/SA_AISoundRange.SA_AISoundRange" null null null)
  (`self.SetRushSetting`)
  (`self.LaunchCharacter` (* (`self.GetActorForwardVector`) 1500.0))
  (`KismetSystemLibrary.Delay` 0.7)
  (`self.SetDefaultSetting`)
  (`self.OnRushEnd`))

(event `AutoDeleteStatue`
  ; SummonStatue
  (`KismetSystemLibrary.PrintString` "Statue Deleted")
  (`/Engine/EditorBlueprintResources/StandardMacros.IsValid` (stale `SummonStatue` _returnvalue)
    (:`Is Valid`
      (`self.K2_DestroyActor` (stale `SummonStatue` _returnvalue)))
    (:`Is Not Valid`
      _))
  (set `self.bCanSummonStatue` true)
  (`BlackboardComponent.SetValueAsBool` (`AIController.Blackboard` (`self.AIController`)) "bCanSummonStatue" true))

(event `ReadyToRush`
  ; Rush
  (`|PlayMontage` (`self.Mesh`) "/Game/KSH/Animations/Montages/AM_Howling.AM_Howling"
    (:`OnCompleted`
      _)
    (:`OnInterrupted`
      _))
  (`self.OnReadyToRushEnd`))

(event `self.ReceiveBeginPlay`
  (`|ExecutionSequence`
    (:`then_0`
      (`PrimitiveComponent.SetCollisionEnabled` (`self.RushCapsule`) "NoCollision")
      (bind _returnvalue (`|CreateWidget` "/Game/KSH/WBP/WBP_BossHealthBar.WBP_BossHealthBar_C"))
      (bind _output_get (set `self.HealthBarRef` _returnvalue))
      (`UserWidget.AddToViewport` _output_get 0))
    (:`then_1`
      (add `self.OnDieEnd` (delegate `DeleteActor`)))))

(event `DeleteActor`
  (`Widget.SetVisibility` (`self.HealthBarRef`) "Collapsed")
  (`BrainComponent.StopLogic` (`AIController.BrainComponent` (`self.AIController`)) "Boss Died")
  (`self.SetLifeSpan` 2.0))

(event `SummonAlter`
  (bind _alterlocation (`self.AlterLocation`))
  ; SummonAlter
  (`GameplayStatics.PlaySoundAtLocation` "/Game/Fab/Sound/Enemy/Boss_Roar.Boss_Roar" (`self.K2_GetActorLocation`) (struct) 1.0 1.0 0.0 "/Game/KSH/Sounds/Attenuation/SA_AISoundRange.SA_AISoundRange" null null null)
  (`|PlayMontage` (`self.Mesh`) "/Game/KSH/Animations/Montages/AM_SummonStatue.AM_SummonStatue"
    (:`OnCompleted`
      _)
    (:`OnInterrupted`
      _))
  (`self.OnSummonAlterEnd`)
  (set `self.AlterLocation` (`self.K2_GetActorLocation` (`self.SpawnAlterLocation`)))
  (bind _returnvalue (`|SpawnActorFromClass` "/Game/KSH/Actors/BP_Alter.BP_Alter_C" (`KismetMathLibrary.MakeTransform` _alterlocation (struct :`Yaw` 180.0)) "Undefined" "MultiplyWithRoot" null null))
  (`KismetSystemLibrary.Delay` 0.2)
  (`GameplayStatics.SpawnEmitterAtLocation` "/Game/StarterContent/Particles/P_Explosion.P_Explosion" _alterlocation (struct) (10.0 10.0 10.0))
  (set `self.bCanSummonAlter` false)
  (`BlackboardComponent.SetValueAsBool` (`AIController.Blackboard` (`self.AIController`)) "bCanSummonAlter" false)
  (`KismetSystemLibrary.K2_SetTimerDelegate` (delegate `AutoDeleteAlter`) 30.0))

(event `Stun`
  ; Stun
  (`|PlayMontage` (`self.Mesh`) "/Game/KSH/Animations/Montages/AM_Stun.AM_Stun"
    (:`OnCompleted`
      _)
    (:`OnInterrupted`
      _))
  (`self.OnStunEnd`))

(event `self.RushCapsule.OnComponentBeginOverlap`
  (params (OverlappedComponent :type "PrimitiveComponent Object Reference") (OtherActor :type "Actor Object Reference") (OtherComp :type "PrimitiveComponent Object Reference") (OtherBodyIndex :type Integer) (bFromSweep :type Boolean) (SweepResult :type "HitResult Structure (by ref)"))
  (if (== OtherActor (`GameplayStatics.GetPlayerCharacter` 0))
    (`KismetSystemLibrary.PrintString` "Player Hitted")
    (`GameplayStatics.ApplyDamage` OtherActor 30.0)))

(event `AutoDeleteAlter`
  ; SummonAlter
  (`KismetSystemLibrary.PrintString` "Alter Deleted")
  (`/Engine/EditorBlueprintResources/StandardMacros.IsValid` (stale `SummonAlter` _returnvalue)
    (:`Is Valid`
      (`self.K2_DestroyActor` (stale `SummonAlter` _returnvalue)))
    (:`Is Not Valid`
      _))
  (set `self.bCanSummonAlter` true)
  (`BlackboardComponent.SetValueAsBool` (`AIController.Blackboard` (`self.AIController`)) "bCanSummonAlter" true))

(fn `SetDefaultSetting`
  (bind _charactermovement (`self.CharacterMovement`))
  (set `CharacterMovementComponent.BrakingFrictionFactor` 2.0 _charactermovement)
  (set `CharacterMovementComponent.BrakingDecelerationWalking` 2048.0 _charactermovement)
  (set `CharacterMovementComponent.GroundFriction` 8.0 _charactermovement)
  (`CharacterMovementComponent.SetMovementMode` _charactermovement "MOVE_Walking" 0)
  (`PrimitiveComponent.SetCollisionEnabled` (`self.RushCapsule`) "NoCollision")
  (`KismetSystemLibrary.PrintString` "Rush Collision Disabled"))

(fn `SetRushSetting`
  (bind _charactermovement (`self.CharacterMovement`))
  (set `CharacterMovementComponent.BrakingFrictionFactor` 0.0 _charactermovement)
  (set `CharacterMovementComponent.BrakingDecelerationWalking` 0.0 _charactermovement)
  (set `CharacterMovementComponent.GroundFriction` 0.0 _charactermovement)
  (`CharacterMovementComponent.SetMovementMode` _charactermovement "MOVE_Falling" 0)
  (`PrimitiveComponent.SetCollisionEnabled` (`self.RushCapsule`) "QueryOnly")
  (`KismetSystemLibrary.PrintString` "Rush Collision Enabled"))

(fn `UserConstructionScript`)