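; BP_Native is an AI Blueprint that switches between human and wolf forms with the sky's day, night and eclipse cycle.
; After a short startup delay it finds the DynamicSky actor, binds its events and sets the initial form from whether it is night.
; Night and eclipse totality trigger Wolf, while day and totality end trigger Human, all through ServerChangeForm.
; EndPlay unbinds the sky events.
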(event `self.ReceiveBeginPlay`
  (bind _skyref (`self.SkyRef`))
  (`parent.ReceiveBeginPlay`)
  (`KismetSystemLibrary.Delay` 0.2)
  (bind _returnvalue (`GameplayStatics.GetActorOfClass` "/Script/Wolf_Island.DynamicSky"))
  (set `self.SkyRef` _returnvalue)
  (add `DynamicSky.OnDayStarted` _skyref (delegate `Change to HumanForm`))
  (add `DynamicSky.OnNightStarted` _skyref (delegate `Change to WolfForm`))
  (add `DynamicSky.OnEclipseTotalityStarted` _skyref (delegate `Change to WolfForm_Eclipse`))
  (add `DynamicSky.OnEclipseTotalityEnded` _skyref (delegate `Change to HumanForm_Eclipse`))
  (if (`DynamicSky.bIsCurrentlyNight` _skyref)
    (`self.ServerChangeForm` "Wolf")
    (else
      (`self.ServerChangeForm` "Human"))))

(event `Change to WolfForm`
  (`self.ServerChangeForm` "Wolf"))

(event `Change to WolfForm_Eclipse`
  (`self.ServerChangeForm` "Wolf"))

(event `Change to HumanForm`
  (`self.ServerChangeForm` "Human"))

(event `Change to HumanForm_Eclipse`
  (`self.ServerChangeForm` "Human"))

(event `self.ReceiveEndPlay`
  (params (EndPlayReason :type "EEndPlayReason Enum" :default "Destroyed"))
  (bind _skyref (`self.SkyRef`)
    (:`then`
      (remove `DynamicSky.OnDayStarted` _skyref (delegate `Change to HumanForm`))
      (remove `DynamicSky.OnNightStarted` _skyref (delegate `Change to WolfForm`))
      (remove `DynamicSky.OnEclipseTotalityStarted` _skyref (delegate `Change to WolfForm_Eclipse`))
      (remove `DynamicSky.OnEclipseTotalityEnded` _skyref (delegate `Change to HumanForm_Eclipse`))
      (`parent.ReceiveEndPlay` EndPlayReason))
    (:`else`)))

(fn `UserConstructionScript`)