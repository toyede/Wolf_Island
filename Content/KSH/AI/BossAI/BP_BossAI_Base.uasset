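; Base boss AI character that exposes attack, howl, rush and knockdown actions plus movement speed control.
; Each action plays a montage and fires its end dispatcher on completion or interruption, though Rush has no montage assigned.
; Capsule overlap with BP_TempWall sets a collision flag on the Blackboard, and any end overlap clears it.
; SetMovementSpeed maps AI state to walk speed, while HP and patrol route getters are empty stubs.
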(event `self.ReceiveBeginPlay`)

(event `Attack`
  (`|PlayMontage` (`self.Mesh`) "/Game/KSH/Animations/AM_Claw.AM_Claw"
    (:`OnCompleted`
      _)
    (:`OnInterrupted`
      _))
  (`self.OnAttackEnd`))

(event `Howling`
  (`|PlayMontage` (`self.Mesh`) "/Game/KSH/Animations/AM_Howling.AM_Howling"
    (:`OnCompleted`
      _)
    (:`OnInterrupted`
      _))
  (`self.OnHowlingEnd`))

(event `Rush`
  (`|PlayMontage` (`self.Mesh`)
    (:`OnCompleted`
      _)
    (:`OnInterrupted`
      _))
  (`self.OnRushEnd`))

(event `KnockedDown`
  (`|PlayMontage` (`self.Mesh`) "/Game/KSH/AI/BossAI/AM_KnockedDown.AM_KnockedDown"
    (:`OnCompleted`
      _)
    (:`OnInterrupted`
      _))
  (`self.OnKnockDownEnd`))

(event `self.CapsuleComponent.OnComponentBeginOverlap`
  (params (OverlappedComponent :type "PrimitiveComponent Object Reference") (OtherActor :type "Actor Object Reference") (OtherComp :type "PrimitiveComponent Object Reference") (OtherBodyIndex :type Integer) (bFromSweep :type Boolean) (SweepResult :type "HitResult Structure (by ref)"))
  (if (== (`GameplayStatics.GetObjectClass` OtherActor) "/Game/KSH/BP_TempWall.BP_TempWall_C")
    (`BlackboardComponent.SetValueAsBool` (`AIController.Blackboard` (`AIBlueprintHelperLibrary.GetAIController` self)) (`self.bIsCollidedKey`) true)))

(event `self.CapsuleComponent.OnComponentEndOverlap`
  (params (OverlappedComponent :type "PrimitiveComponent Object Reference") (OtherActor :type "Actor Object Reference") (OtherComp :type "PrimitiveComponent Object Reference") (OtherBodyIndex :type Integer))
  (`BlackboardComponent.SetValueAsBool` (`AIController.Blackboard` (`AIBlueprintHelperLibrary.GetAIController` self)) (`self.bIsCollidedKey`) false))

(fn `GetCurrentHp`
  (returns (CurrentHp :type "Float (double-precision)"))
  (return 0.0))

(fn `GetPatrolRoute`
  (returns (PatrolRoute :type "/Game/KSH/AI/WolfAI/BP_PatrolRoute Object Reference"))
  (return null))

(fn `SetMovementSpeed`
  (params (State :type "/Game/KSH/AI/Enums_AI/E_BossAIState Enum" :default "NewEnumerator0"))
  (set `CharacterMovementComponent.MaxWalkSpeed` (select `/Game/KSH/AI/Enums_AI/E_BossAIState` State :`NewEnumerator2` 100.0 :`NewEnumerator3` 300.0 :`NewEnumerator4` 500.0 :`NewEnumerator5` 2000.0) (`self.CharacterMovement`))
  (return))

(fn `UserConstructionScript`)