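; Base wolf AI Blueprint for a werewolf enemy that can attack, howl and switch between human and wolf forms.
; Attack and Howling play montages and fire end dispatchers on either completion or interruption.
; SwitchForm swaps the skeletal mesh between mannequin and werewolf, toggles IsWolf and broadcasts the change; its OnRep function is empty.
; It initializes health on BeginPlay and exposes getters for current HP and patrol route.
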(event `self.ReceiveBeginPlay`
  (bind _output_get (set `self.MaxHp` 100.0))
  (set `self.CurrentHp` _output_get))

(event `Attack`
  (`|PlayMontage` (`self.Mesh`) "/Game/KSH/Animations/AM_Claw.AM_Claw"
    (:`OnCompleted`
      _)
    (:`OnInterrupted`
      _))
  (`self.OnAttackEnd`))

(event `Howling`
  (`|PlayMontage` (`self.Mesh`) "/Game/KSH/Animations/AM_Howling.AM_Howling"
    (:`OnCompleted`
      _)
    (:`OnInterrupted`
      _))
  (`self.OnHowlingEnd`))

(event `SwitchForm`
  (bind _mesh (`self.Mesh`))
  (if (`self.bIsWolf`)
    (`SkeletalMeshComponent.SetSkeletalMeshAsset` _mesh "/Game/Characters/Mannequin_UE4/Meshes/SK_Mannequin.SK_Mannequin")
    (bind _output_get (set `self.bIsWolf` false))
    (`self.OnFormChanged` _output_get)
    (else
      (`SkeletalMeshComponent.SetSkeletalMeshAsset` _mesh "/Game/Werewolf/Mesh/Full/SK_Werewolf_Full1.SK_Werewolf_Full1")
      (bind _output_get_2 (set `self.bIsWolf` true))
      (`self.OnFormChanged` _output_get_2))))

(fn `GetCurrentHp`
  (returns (CurrentHp :type "Float (double-precision)"))
  (return (`self.CurrentHp`)))

(fn `GetPatrolRoute`
  (returns (PatrolRoute :type "/Game/KSH/AI/WolfAI/BP_PatrolRoute Object Reference"))
  (return (`self.PatrolRoute`)))

(fn `OnRep_bIsWolf`)

(fn `UserConstructionScript`)