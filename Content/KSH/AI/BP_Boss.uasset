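; BP_Boss is a boss Blueprint that manages the on-screen boss health bar during combat.
; When combat starts, it creates a WBP_BossHpBar for the first player controller if it is local, passes it the boss reference and adds it to the viewport.
; When combat ends, it removes and clears the widget after a short delay.
; EndPlay is empty, and a similar cleanup chain that calls parent EndPlay is left unconnected.
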(event `self.OnCombatStarted`
  (params (Boss :type "EnemyAIBoss Object Reference"))
  (bind _returnvalue (`GameplayStatics.GetPlayerController` 0))
  (if (`Controller.IsLocalPlayerController` _returnvalue)
    (bind _returnvalue_2 (`|CreateWidget` "/Game/KSH/UI/WBP_BossHpBar.WBP_BossHpBar_C" _returnvalue Boss))
    (bind _output_get (set `self.BossHpBarWidget` _returnvalue_2))
    (set `/Game/KSH/UI/WBP_BossHpBar.BossRef` Boss _output_get)
    (`UserWidget.AddToViewport` _returnvalue_2 0)))

(event `self.OnCombatEnded`
  (bind _bosshpbarwidget (`self.BossHpBarWidget`)
    (:`then`
      (`KismetSystemLibrary.Delay` 1.5)
      (`Widget.RemoveFromParent` _bosshpbarwidget)
      (set `self.BossHpBarWidget` null))
    (:`else`)))

(event `self.ReceiveEndPlay`
  (params (EndPlayReason :type "EEndPlayReason Enum" :default "Destroyed")))

(fn `UserConstructionScript`)