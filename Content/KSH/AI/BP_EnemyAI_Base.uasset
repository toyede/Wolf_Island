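; Base enemy AI character that takes damage through its StatusComponent and performs a melee claw attack.
; The attack montage's notify triggers a forward sphere trace that damages a hit pawn, ignoring fellow enemies gathered at BeginPlay, and completion or interruption fires OnAttackEnd.
; SetMovementSpeed maps AI state to walk speed.
; GetCurrentHp and GetPatrolRoute are empty stubs here.
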(event `self.ReceiveBeginPlay`
  (bind _outactors (`GameplayStatics.GetAllActorsOfClass` "BP_EnemyAI_Base_C"))
  (set `self.Actors to Ignore` _outactors))

(event `self.ReceiveAnyDamage`
  (params (Damage :type "Float (single-precision)") (DamageType :type "DamageType Object Reference") (InstigatedBy :type "Controller Object Reference") (DamageCauser :type "Actor Object Reference"))
  (`StatusComponent.DecreaseHP` (`self.StatusComponent`) Damage))

(event `Attack`
  (bind _notifyname (`|PlayMontage` (`self.Mesh`) "/Game/KSH/Animations/Montages/AM_Claw.AM_Claw")
    (:`OnCompleted`
      (`self.OnAttackEnd` :!label _label))
    (:`OnInterrupted`
      (goto _label))
    (:`OnNotifyBegin`
      (switch `name` _notifyname
        (:`Attack`
          (bind (_outhit _returnvalue) (`KismetSystemLibrary.SphereTraceSingleForObjects` (+ (`self.K2_GetActorLocation`) (* (`self.GetActorForwardVector`) 100.0)) (+ (`self.K2_GetActorLocation`) (* (`self.GetActorForwardVector`) 150.0)) 20.0 (`|MakeArray` "ObjectTypeQuery3" :!type "EObjectTypeQuery Enum") false (`self.Actors to Ignore`) "ForDuration"))
          (if _returnvalue
            (`GameplayStatics.ApplyDamage` (`.HitActor` (`GameplayStatics.BreakHitResult` _outhit)) (`self.AttackDamage`) (`self.GetController`) self)))))))

(fn `GetCurrentHp`
  (returns (CurrentHp :type "Float (double-precision)"))
  (return 0.0))

(fn `GetPatrolRoute`
  (returns (PatrolRoute :type "Actor Object Reference"))
  (return null))

(fn `SetMovementSpeed`
  (params (State :type "EEnemyState Enum" :default "None"))
  (set `CharacterMovementComponent.MaxWalkSpeed` (select `EEnemyState` State :`Passive` 200.0 :`Attacking` 600.0 :!type "Float (single-precision)") (`self.CharacterMovement`))
  (return))

(fn `UserConstructionScript`)