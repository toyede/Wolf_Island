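; BP_DynamicSky_ver4 is a sky actor that plays a timed eclipse when RequestEclipseStart or StartEclipse is called.
; A timeline drives the sky sphere material's eclipse offset and active flag, along with the sun directional light's intensity.
; Timeline event tracks fire dispatchers at totality start and end.
; On finish, it clears the eclipse flags and calls ServerSetEclipseOccurred on the EclipseManager.
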(event `StartEclipse`
  (bind (_direction _eclipseoffset _sunbrightness) (`Timeline|타임라인`)
    (:`Update`
      (`MeshComponent.SetScalarParameterValueOnMaterials` (`self.SkySphereMesh`) "IsEclipseActive" 1.0)
      (`MeshComponent.SetScalarParameterValueOnMaterials` (`self.SkySphereMesh`) "EclipseOffset" _eclipseoffset)
      (`LightComponent.SetIntensity` (`self.SunDirectionalLight`) _sunbrightness))
    (:`Finished`
      (set `self.bEclipseTriggered` false)
      (`MeshComponent.SetScalarParameterValueOnMaterials` (`self.SkySphereMesh`) "IsEclipseActive" 0.0)
      (`EclipseManagerComponent.Server_SetEclipseOccurred` (`self.EclipseManager`)))
    (:`TotalityStart`
      (`self.OnEclipseTotalityStarted`))
    (:`TotalityEnd`
      (`self.OnEclipseTotalityEnded`))))

(event `self.BP_RequestEclipseStart`
  (`self.StartEclipse`))

(fn `UserConstructionScript`)