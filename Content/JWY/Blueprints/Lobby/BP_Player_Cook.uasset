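; Player cook character Blueprint with inventory UI, an emote montage, a self-only scene capture and master-pose mesh setup.
; Damage feeds StatusComponent, with wolf attacks starting infection; death disables input and ragdolls the mesh.
; A test Infected event ragdolls, then resets time of day and respawns at PlayerStart, but its infection-change binding is disconnected.
; Debug keys save/load the world, destroy traced actors, and print chest inventories and infection state.
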(event Custom|Fuckyou
  (Animation|Montage|PlayMontage (Variables|Character|GetMesh) "/Game/JSY/Characters/Player/Animation/AM_FuckYou.AM_FuckYou"))

(event Custom|Infected
  (bind _capsulecomponent (Variables|Default|GetCapsuleComponent))
  (bind _mesh (Variables|Character|GetMesh))
  ;[0.15 0.15 0.15 0.5] TEST_KSH
  (Physics|SetSimulatePhysics (Variables|Character|GetMesh) true)
  (Collision|SetCollisionEnabled (Variables|Default|GetCapsuleComponent) "NoCollision")
  (Variables|/Script/Wolf_Island.StatusComponent|SetbIsIncapacitated (Variables|Default|GetStatusComponent) true)
  (Utilities|FlowControl|Delay 5.0)
  (bind _returnvalue (Actor|GetActorOfClass "/Game/KSH/Actors/BP_DynamicSky_KSH.BP_DynamicSky_KSH_C"))
  (Variables|/Game/KSH/Actors/BP_DynamicSky_KSH.BP_DynamicSky_KSH_C|SetTimeOfDay _returnvalue 9.0)
  (bind _returnvalue_2 (Actor|GetActorOfClass "/Script/Engine.PlayerStart"))
  (Transformation|SetActorLocation (Transformation|GetActorLocation _returnvalue_2) false false)
  (Physics|SetSimulatePhysics (Variables|Character|GetMesh) false)
  (Collision|SetCollisionEnabled _capsulecomponent "QueryAndPhysics")
  (Transformation|AttachComponentToComponent _mesh _capsulecomponent "None" "SnapToTarget" "SnapToTarget" "SnapToTarget" true)
  (Transformation|SetRelativeLocationAndRotation _mesh "0.000000,0.000000,-90.000000" "0.000000,-90.000000,0.000000" false false)
  (Variables|/Script/Wolf_Island.StatusComponent|SetbIsIncapacitated (Variables|Default|GetStatusComponent) false))

(event Custom|Emotion
  (CallFunction|Fuckyou))

(event Input|EnhancedActionEvents|EnhancedInputActionIA_Inventory
  (params (ActionValue :type Boolean) (ElapsedSeconds :type Float%20%28double-precision%29) (TriggeredSeconds :type Float%20%28double-precision%29) (InputAction :type Input%20Action%20Object%20Reference :default "/Game/JSY/Characters/Player/Input/IA_Inventory.IA_Inventory"))
  (bind _returnvalue (Game|GetPlayerController 0))
  (bind _returnvalue_2 (UserInterface|CreateWidget "/Game/JSY/Widgets/Inventory/WBP_Inventory.WBP_Inventory_C"))
  (UserInterface|Viewport|AddtoViewport _returnvalue_2 0)
  (Input|SetInputModeUIOnly _returnvalue 0 "DoNotLock" false)
  (Variables|/Script/Engine.PlayerController|SetbShowMouseCursor _returnvalue true))

(event Input|EnhancedActionEvents|EnhancedInputActionIA_Emotion
  (params (ActionValue :type Boolean) (ElapsedSeconds :type Float%20%28double-precision%29) (TriggeredSeconds :type Float%20%28double-precision%29) (InputAction :type Input%20Action%20Object%20Reference :default "/Game/JSY/Characters/Player/Input/IA_Emotion.IA_Emotion"))
  (CallFunction|Emotion))

(event EventBeginPlay
  (Rendering|SceneCapture|ShowOnlyActorComponents (Variables|Default|GetSceneCaptureComponent2D) self false)
  (Class|InventoryComponent|LoadInventory (Variables|Default|GetInventoryComponent)))

(event EventOnDeath
  (bind _as플레이어_컨트롤러 (Utilities|Casting|CastToPlayerController (Pawn|GetController)))
  (Input|DisableInput _as플레이어_컨트롤러)
  (Physics|SetSimulatePhysics (Variables|Character|GetMesh) true))

(event EventTick
  (params (DeltaSeconds :type Float%20%28single-precision%29)))

(event Game|Damage|EventAnyDamage
  (params (Damage :type Float%20%28single-precision%29) (DamageType :type Damage%20Type%20Object%20Reference) (InstigatedBy :type Controller%20Object%20Reference) (DamageCauser :type Actor%20Object%20Reference))
  (bind _statuscomponent (Variables|Default|GetStatusComponent))
  (Class|StatusComponent|DecreaseHP _statuscomponent Damage)
  (if (== (Utilities|GetClass DamageType) "/Game/KSH/DamageType/DamageType_WolfAttack.DamageType_WolfAttack_C")
    (if (not (Variables|/Script/Wolf_Island.StatusComponent|GetIsInfected _statuscomponent))
      (Class|StatusComponent|StartInfection _statuscomponent))))

(event Input|KeyboardEvents|DebugKeyF
  (params (Key :type Key%20Structure :default "None") (ActionValue :type Input%20Action%20Value%20Structure))
  (bind _firstpersoncamera (Variables|Default|GetFirstPersonCamera))
  (bind _returnvalue (Transformation|GetWorldLocation _firstpersoncamera))
  (:Pressed
    (bind _outhit (Collision|LineTraceByChannel _returnvalue (+ _returnvalue (* (Math|Vector|GetForwardVector _firstpersoncamera) 1e+03)) "TraceTypeQuery4" false 0 "ForDuration"))
    (Actor|DestroyActor (.HitActor (Collision|BreakHitResult _outhit)))))

(event Input|KeyboardEvents|DebugKeyZ
  (params (Key :type Key%20Structure :default "None") (ActionValue :type Input%20Action%20Value%20Structure))
  (:Pressed
    (bind _asmain_game_mode (Utilities|Casting|CastToMainGameMode (Game|GetGameMode)))
    (Class|MainGameMode|SaveWorld _asmain_game_mode)
    (Utilities|Casting|CastToMainGameState (Game|GetGameState))))

(event Input|KeyboardEvents|DebugKeyX
  (params (Key :type Key%20Structure :default "None") (ActionValue :type Input%20Action%20Value%20Structure))
  (:Pressed
    (bind _asmain_game_mode (Utilities|Casting|CastToMainGameMode (Game|GetGameMode)))
    (Class|MainGameMode|LoadWorld _asmain_game_mode)
    (bind _asmain_game_state (Utilities|Casting|CastToMainGameState (Game|GetGameState)))
    (Class|MainGameState|AddChattingMessage _asmain_game_state (Utilities|Struct|MakeChattingData "NOTICE" "SYSTEM" "세이브 불러오기" (Class|KismetMathLibrary|ToUnixTimestamp (Math|DateTime|UTCNow))))))

(event Input|KeyboardEvents|DebugKeyR
  (params (Key :type Key%20Structure :default "None") (ActionValue :type Input%20Action%20Value%20Structure))
  (:Pressed
    (bind _outactors (Actor|GetAllActorsOfClass "/Script/Wolf_Island.Chest"))
    (for _array_element _outactors
      (Development|PrintString (Utilities|GetDisplayName _array_element))
      (Class|InventoryComponent|PrintInventory (Variables|/Script/Wolf_Island.Chest|GetInventoryComponent _array_element) 5.0))))

(event Input|KeyboardEvents|T
  (params (Key :type Key%20Structure :default "None"))
  (bind _statuscomponent (Variables|Default|GetStatusComponent))
  (:Pressed
    (Development|PrintString (Utilities|String|ToString(Float) (Variables|/Script/Wolf_Island.StatusComponent|GetCurrentInfectionRate _statuscomponent)))
    (Development|PrintString (Utilities|String|ToString(Boolean) (Variables|/Script/Wolf_Island.StatusComponent|GetIsInfected _statuscomponent)))))

(fn ConstructionScript
  (CallFunction|EnableMasterPose)
  (CallFunction|EnableMasterPose)
  (CallFunction|EnableMasterPose))