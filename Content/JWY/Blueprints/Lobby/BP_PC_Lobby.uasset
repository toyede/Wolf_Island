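; Lobby player controller that creates the lobby UI for the local player and relays that player's lobby actions to the game mode.
; On BeginPlay it shows the cursor, sets game-and-UI input and requests a player info update, which can also be re-requested after a short delay.
; Server-named events toggle ready or set the selected character in PlayerInfo, then notify BP_LobbyGameMode; another asks it to start game travel.
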(event `self.ReceiveBeginPlay`
  (if (`self.IsLocalPlayerController`)
    (bind _returnvalue (`|CreateWidget` "/Game/JWY/Blueprints/UI/W_LobbyUI.W_LobbyUI_C"))
    (bind _output_get (set `self.LobbyUI` _returnvalue))
    (`UserWidget.AddToViewport` _output_get 0)
    (set `self.bShowMouseCursor` true)
    (`WidgetBlueprintLibrary.SetInputMode_GameAndUIEx` self (`self.LobbyUI`))
    (`self.ROS_Update Player Info`)))

(event `Update Player Info`
  (`KismetSystemLibrary.Delay` 0.1)
  (`self.ROS_Update Player Info`))

(event `ROS_Update Player Info`
  (bind _asbp_lobby_game_mode (cast `/Game/JWY/Blueprints/Lobby/BP_LobbyGameMode` (`GameplayStatics.GetGameMode`)))
  (`/Game/JWY/Blueprints/Lobby/BP_LobbyGameMode.Update Player Info` _asbp_lobby_game_mode self))

(event `ROS_ToggleReadyStatus`
  (bind _player_info (`self.Player Info`))
  (setmembers `/Game/JWY/Blueprints/Lobby/S_PlayerInfo` :`StructRef` _player_info :`Ready` (not (`.Ready_10_87DB5E424FCCA6FED9127E862476A4AF` (break `/Game/JWY/Blueprints/Lobby/S_PlayerInfo` _player_info))))
  (bind _asbp_lobby_game_mode (cast `/Game/JWY/Blueprints/Lobby/BP_LobbyGameMode` (`GameplayStatics.GetGameMode`)))
  (`/Game/JWY/Blueprints/Lobby/BP_LobbyGameMode.Update Player Info` _asbp_lobby_game_mode self))

(event `Server_RequestStartGame`
  (bind _asbp_lobby_game_mode (cast `/Game/JWY/Blueprints/Lobby/BP_LobbyGameMode` (`GameplayStatics.GetGameMode`)))
  (`/Game/JWY/Blueprints/Lobby/BP_LobbyGameMode.Run Game Travel` _asbp_lobby_game_mode))

(event `Server_UpdateSelectedCharacter`
  (params (NewIndex :type Integer))
  (setmembers `/Game/JWY/Blueprints/Lobby/S_PlayerInfo` :`StructRef` (`self.Player Info`) :`Selected Character` NewIndex)
  (bind _asbp_lobby_game_mode (cast `/Game/JWY/Blueprints/Lobby/BP_LobbyGameMode` (`GameplayStatics.GetGameMode`)))
  (`/Game/JWY/Blueprints/Lobby/BP_LobbyGameMode.Update Player Info` _asbp_lobby_game_mode self))

(fn `UserConstructionScript`)