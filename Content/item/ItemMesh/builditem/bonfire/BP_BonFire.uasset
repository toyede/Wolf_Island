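; BP_BonFire is an interactable bonfire build item that gives players access to a bonfire UI.
; Interact casts the interactor to BP_MainPlayer and calls its ClientOpenBonfireUI.
; A separate ControllerCheck event creates WBP_BonFire for player controller 0, shows the mouse cursor and sets Game and UI input mode.
; Focus events toggle custom depth on the BonFire component to support highlighting.
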(event `self.Interact`
  (params (Interactor :type "Actor Object Reference"))
  (bind _asbp_main_player (cast `/Game/JSY/Characters/Player/BP_MainPlayer` Interactor))
  (`MainPlayer.Client_OpenBonfireUI` _asbp_main_player))

(event `ControllerCheck`
  (bind _returnvalue (`GameplayStatics.GetPlayerController` 0))
  (bind _returnvalue_2 (`|CreateWidget` "/Game/JSY/Widgets/Craft/WBP_BonFire.WBP_BonFire_C" _returnvalue))
  (`UserWidget.AddToViewport` _returnvalue_2 0)
  (set `PlayerController.bShowMouseCursor` true _returnvalue)
  (`WidgetBlueprintLibrary.SetInputMode_GameAndUIEx` _returnvalue null))

(event `InteractionInterface.BeginFocus`
  (`PrimitiveComponent.SetRenderCustomDepth` (`self.BonFire`) true))

(event `InteractionInterface.EndFocus`
  (`PrimitiveComponent.SetRenderCustomDepth` (`self.BonFire`) false))

(fn `UserConstructionScript`)