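; BP_BrokenShip is an interactable broken boat that shows its repair progress through body, anchor and radar flags.
; BeginPlay calls CompleteRepair, then sets propeller, AC and RD component visibility from those flags, swapping in the fixed hull mesh when IsBody is true.
; Interact has the player open the repair UI client-side for this ship.
; UpdateShipVisuals only reveals repaired parts; the RepairShip event handler is empty and unbound.
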(event `self.ReceiveBeginPlay`
  (`self.CompleteRepair` self)
  (`|ExecutionSequence`
    (:`then_0`
      (if (`self.bIsBody`)
        (`SceneComponent.SetVisibility` (`self.Propeller`) true true)
        (`StaticMeshComponent.SetStaticMesh` (`self.BrokenShip`) "/Game/item/ItemMesh/boat/boat_fixed/SM_boat_fixed.SM_boat_fixed")
        (else
          (`SceneComponent.SetVisibility` (`self.Propeller`) false true))))
    (:`then_1`
      (if (`self.bIsAnchor`)
        (`SceneComponent.SetVisibility` (`self.AC`) true true)
        (else
          (`SceneComponent.SetVisibility` (`self.AC`) false true))))
    (:`then_2`
      (if (`self.bIsRadar`)
        (`SceneComponent.SetVisibility` (`self.RD`) true true)
        (else
          (`SceneComponent.SetVisibility` (`self.RD`) false true))))))

(event `self.Interact`
  (params (Interactor :type "Actor Object Reference"))
  (`|ExecutionSequence`
    (:`then_0`
      (bind _asbp_main_player (cast `/Game/JSY/Characters/Player/BP_MainPlayer` Interactor))
      (`MainPlayer.Client_OpenRepairUI` _asbp_main_player self)
      (`KismetSystemLibrary.PrintString` (`KismetStringLibrary.Conv_BoolToString` (`self.bIsBody`))))))

(event `self.UpdateShipVisuals`
  (`|ExecutionSequence`
    (:`then_0`
      (if (`self.bIsBody`)
        (`SceneComponent.SetVisibility` (`self.Propeller`) true true)
        (`StaticMeshComponent.SetStaticMesh` (`self.BrokenShip`) "/Game/item/ItemMesh/boat/boat_fixed/SM_boat_fixed.SM_boat_fixed")))
    (:`then_1`
      (if (`self.bIsAnchor`)
        (`SceneComponent.SetVisibility` (`self.AC`) true true)))
    (:`then_2`
      (if (`self.bIsRadar`)
        (`SceneComponent.SetVisibility` (`self.RD`) true true)))))

(event `RepairShip_이벤트`)

(fn `UserConstructionScript`)