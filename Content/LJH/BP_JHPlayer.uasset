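; BP_JHPlayer is a player character Blueprint whose only active logic is on-screen debugging of interaction and movement state.
; Each Tick prints the current interactable's name, the interaction timer's elapsed time and whether the character is falling, each lasting one frame.
; BeginPlay and the construction script are empty, and the code that adds WBP_TestHUD to the viewport is disconnected.
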(event EventBeginPlay)

(event Collision|EventActorBeginOverlap
  (params (OtherActor :type Actor%20Object%20Reference)))

(event EventTick
  (params (DeltaSeconds :type Float%20%28single-precision%29))
  (Development|PrintString (Utilities|GetDisplayName (.CurrentInteractable (Utilities|Struct|BreakInteractionData (Variables|Default|GetInteractionData)))) true true "(R=0.000000,G=0.660000,B=1.000000,A=1.000000)" DeltaSeconds)
  (Development|PrintString (Utilities|String|ToString(Float) (Class|KismetSystemLibrary|GetTimerElapsedTimeHandle (Variables|Default|GetInteractionTimer))) true true "(R=1.000000,G=0.000000,B=0.240346,A=1.000000)" DeltaSeconds)
  (Development|PrintString (Utilities|String|ToString(Boolean) (AI|Components|NavMovement|IsFalling (Variables|Character|GetCharacterMovement))) true true "(R=1.000000,G=0.893594,B=0.000000,A=1.000000)" DeltaSeconds))

(event Input|KeyboardEvents|DebugKeyP
  (params (Key :type Key%20Structure :default "None") (ActionValue :type Input%20Action%20Value%20Structure)))

(fn ConstructionScript)