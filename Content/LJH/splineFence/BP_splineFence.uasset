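; BP_splineFence is a construction-time tool that lays copies of a fence mesh along a spline.
; The construction script divides the spline length by the X extent of the Fence mesh's bounding box to set the segment count.
; It adds a static mesh component at each interval, using the spline's local transform at that distance without spline scale, so pieces follow the curve without bending.
; The event graph holds no active logic.
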(fn `UserConstructionScript`
  (bind (_returnvalue_min _returnvalue_max) (break `Box` (`StaticMesh.GetBoundingBox` (`self.Fence`))))
  (bind _returnvalue_x (`KismetMathLibrary.BreakVector` (- _returnvalue_max _returnvalue_min)))
  (for _index (range (+ (`KismetMathLibrary.FTrunc` (/ (`SplineComponent.GetSplineLength` (`self.Spline`)) _returnvalue_x)) 1))
    (bind _returnvalue (`AddComponent|NODE_AddStaticMeshComponent-2` :`RelativeTransform` (`SplineComponent.GetTransformAtDistanceAlongSpline` (`self.Spline`) (* _index _returnvalue_x) "Local" false)))
    (`StaticMeshComponent.SetStaticMesh` _returnvalue (`self.Fence`))))